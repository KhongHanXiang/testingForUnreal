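; BP_SoccorGoal is a soccer goal actor that detects the ball and resets it after a score.
; On BeginPlay it stores the referenced ball's starting location as the respawn transform.
; When a BP_SoccorBall overlaps its Box, it plays a hit particle above the goal at a fixed world height and destroys the ball.
; After a short delay it spawns a new ball at the stored location.
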(event `self.ReceiveBeginPlay`
  (bind _soccorballref (`self.SoccorBallRef`))
  (`/Engine/EditorBlueprintResources/StandardMacros.IsValid` _soccorballref
    (:`Is Valid`
      (set `self.BallSpawnLocation` (`KismetMathLibrary.Conv_VectorToTransform` (`self.K2_GetActorLocation` _soccorballref))))))

(event `self.Box.OnComponentBeginOverlap`
  (params (OverlappedComponent :type "PrimitiveComponent Object Reference") (OtherActor :type "Actor Object Reference") (OtherComp :type "PrimitiveComponent Object Reference") (OtherBodyIndex :type Integer) (bFromSweep :type Boolean) (SweepResult :type "HitResult Structure (by ref)"))
  (bind _asbp_soccor_ball (cast `/Game/Blueprints/SoccerBlueprints/BP_SoccorBall` OtherActor))
  (`GameplayStatics.SpawnEmitterAtLocation` "/Game/FXVarietyPack/Particles/P_ky_hit1.P_ky_hit1" (`KismetMathLibrary.MakeVector` (.x (`SceneComponent.K2_GetComponentLocation` (`self.SoccorGoal`))) (.y (`SceneComponent.K2_GetComponentLocation` (`self.SoccorGoal`))) 300.0))
  (`self.K2_DestroyActor` _asbp_soccor_ball)
  (`KismetSystemLibrary.Delay` 2.0)
  (`|SpawnActorFromClass` "/Game/Blueprints/SoccerBlueprints/BP_SoccorBall.BP_SoccorBall_C" (`self.BallSpawnLocation`) "Undefined" "OverrideRootScale" null null))

(fn `UserConstructionScript`)